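; Spawner actor that places food (Bp_Eat) and pickups (Bp_Haste, Bp_Teleportator) at random XY points within a square area at a fixed height.
; On BeginPlay it spawns one food item and binds to its OnDestroyed, so each destroyed food immediately spawns a replacement.
; Two looping timers independently spawn haste pickups frequently and teleporters less often, with no cap on how many accumulate.
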(event Custom|Spawn%20Eat
  (bind _returnvalue (Game|SpawnActorfromClass "/Game/Blueprints/Bp_Eat.Bp_Eat_C" (Math|Transform|MakeTransform (Math|Vector|MakeVector (Math|Random|RandomFloatinRange -8e+02 8e+02) (Math|Random|RandomFloatinRange -8e+02 8e+02) -1e+02) "0, 0, 0" "1.000000,1.000000,1.000000") "Undefined" "MultiplyWithRoot" 0 0))
  (Game|BindEventtoOnDestroyed _returnvalue (delegate Custom|EatDestroyed)))

(event Custom|Spawn%20Haste
  (Game|SpawnActorfromClass "/Game/Blueprints/Bp_Haste.Bp_Haste_C" (Math|Transform|MakeTransform (Math|Vector|MakeVector (Math|Random|RandomFloatinRange -8e+02 8e+02) (Math|Random|RandomFloatinRange -8e+02 8e+02) -1e+02) "0, 0, 0" "1.000000,1.000000,1.000000") "Undefined" "MultiplyWithRoot" 0 0))

(event Custom|EatDestroyed
  (params (DestroyedActor :type Actor%20Object%20Reference))
  (CallFunction|SpawnEat))

(event Custom|SpawnTeleport
  (Game|SpawnActorfromClass "/Game/Blueprints/Bp_Teleportator.Bp_Teleportator_C" (Math|Transform|MakeTransform (Math|Vector|MakeVector (Math|Random|RandomFloatinRange -8e+02 8e+02) (Math|Random|RandomFloatinRange -8e+02 8e+02) -1e+02) "0, 0, 0" "1.000000,1.000000,1.000000") "Undefined" "MultiplyWithRoot" 0 0))

(event EventBeginPlay
  (CallFunction|SpawnEat)
  (Utilities|Time|SetTimerbyEvent (delegate Custom|Spawn%20Haste) 5.0 true)
  (Utilities|Time|SetTimerbyEvent (delegate Custom|SpawnTeleport) 3e+01 true))

(fn ConstructionScript)